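; Base-style interactable actor with a configurable skeletal or static mesh, sphere trigger and widget prompt.
; The construction script applies the meshes, trigger radius and component offsets; BeginPlay passes the description to the Interact_UI widget.
; Trigger overlaps toggle input and register or unregister the actor with PlayerCharacter_BP.
; ToggleUI sets prompt visibility, while Interact and left/right mouse handlers are stubs storing the character, with Interact also printing debug text.
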(event OnComponentBeginOverlap(InteractTrigger)
  (params (OverlappedComponent :type Primitive%20Component%20Object%20Reference) (OtherActor :type Actor%20Object%20Reference) (OtherComp :type Primitive%20Component%20Object%20Reference) (OtherBodyIndex :type Integer) (bFromSweep :type Boolean) (SweepResult :type Hit%20Result%20Structure%20%28by%20ref%29))
  (bind _asplayer_character_bp (Utilities|Casting|CastToPlayerCharacter_BP OtherActor))
  (Input|EnableInput (Game|GetPlayerController 0))
  (Default|AddInteraction _asplayer_character_bp self))

(event OnComponentEndOverlap(InteractTrigger)
  (params (OverlappedComponent :type Primitive%20Component%20Object%20Reference) (OtherActor :type Actor%20Object%20Reference) (OtherComp :type Primitive%20Component%20Object%20Reference) (OtherBodyIndex :type Integer))
  (bind _asplayer_character_bp (Utilities|Casting|CastToPlayerCharacter_BP OtherActor))
  (Input|DisableInput (Game|GetPlayerController 0))
  (Default|RemoveInteraction _asplayer_character_bp self))

(event EventBeginPlay
  (Utilities|FlowControl|Sequence
    (:then_0
      (bind _asinteract_ui (Utilities|Casting|CastToInteract_UI (UserInterface|GetUserWidgetObject (Variables|Default|GetInteract_UI))))
      (bind _output_get (Variables|Default|SetInteractionUIWidget _asinteract_ui))
      (Default|SetInteractDescription _output_get (Variables|Default|GetInteract%20Description%20)))))

(fn ConstructionScript
  (Setup|SetupMesh)
  (Setup|SetupTrigger)
  (Setup|SetupUI))

(fn ToggleUI
  (params (Visible? :type Boolean))
  (Rendering|SetVisibility (Variables|Default|GetInteract_UI) Visible? false))

(fn Interact
  (params (Character :type Playercharacter%20Object%20Reference))
  (Variables|Default|SetInteractCharacter Character)
  (Development|PrintString "Interacted"))

(fn SetupMesh
  (Class|SkinnedMeshComponent|SetSkeletalMesh (Variables|Default|GetInteractMesh) (Variables|Default|GetInteractionMesh) true)
  (Components|StaticMesh|SetStaticMesh (Variables|Default|GetInteractMeshST) (Variables|Default|GetInteractionMeshS))
  (Transformation|SetRelativeTransform (Variables|Default|GetInteractMeshST) (Variables|Default|GetMeshTransform) false false))

(fn SetupTrigger
  (Components|Sphere|SetSphereRadius (Variables|Default|GetInteractTrigger) (Variables|Default|GetTriggerRadius) true)
  (Transformation|SetRelativeLocation (Variables|Default|GetInteractTrigger) (Variables|Default|GetTriggerLocation) false false))

(fn SetupUI
  (Transformation|SetRelativeLocation (Variables|Default|GetInteract_UI) (Variables|Default|GetUI%20Location) false false))

(fn InteractLeftMouse
  (params (Character :type Playercharacter%20Object%20Reference))
  (Variables|Default|SetInteractCharacter Character))

(fn InteractRightMouse
  (params (Character :type Playercharacter%20Object%20Reference))
  (Variables|Default|SetInteractCharacter Character))