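; Player character Blueprint that handles interaction targeting and routes inventory and hand-item input.
; A looping short timer picks the registered interaction best aligned with the camera by dot product against a threshold, skipping this while falling, and toggles its UI.
; Interact triggers that selection, and Pocket opens a widget.
; Mouse wheel, Inventory and left click forward messages to the current bag or held actor stored in the GameInstance.
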(event Custom|100ms
  (Utilities|FlowControl|Sequence
    (:then_0
      (Interaction|UpdateInteraction))))

(event EventBeginPlay
  (bind _returnvalue (Utilities|Time|SetTimerbyEvent (delegate Custom|100ms) 0.1 true))
  (Variables|Default|SetShortTick _returnvalue))

(event EventTick
  (params (DeltaSeconds :type Float%20%28single-precision%29))
  (Variables|Default|SetDelta DeltaSeconds))

(event Input|ActionEvents|InputActionInteract
  (params (Key :type Key%20Structure))
  (:Pressed
    (bind _selected_interaction (Variables|Default|GetSelected%20Interaction)
      (:then
        (Default|Interact _selected_interaction self))
      (:else))))

(event Input|ActionEvents|InputActionInventory
  (params (Key :type Key%20Structure))
  (:Pressed
    (bind _asnon_game_instance_bp (Utilities|Casting|CastToNon_GameInstance_BP (Game|GetGameInstance)))
    (Class|Pickup|Inventory(Message) (Variables|/Game/Blueprints/NoN_GameInstance_BP.Non_GameInstance_BP_C|GetCurrentBag _asnon_game_instance_bp))))

(event Input|ActionEvents|InputActionPocket
  (params (Key :type Key%20Structure))
  (:Pressed
    (bind _returnvalue (UserInterface|CreateWidget "/Game/Blueprints/PocketUI.PocketUI_C"))
    (UserInterface|Viewport|AddtoViewport _returnvalue 0)))

(event Input|MouseEvents|LeftMouseButton
  (params (Key :type Key%20Structure))
  (:Pressed
    (bind _asnon_game_instance_bp (Utilities|Casting|CastToNon_GameInstance_BP (Game|GetGameInstance)))
    (Class|Pickup|LeftMouseButton(Message) (Variables|/Game/Blueprints/NoN_GameInstance_BP.Non_GameInstance_BP_C|GetActorInHand _asnon_game_instance_bp))))

(event Input|KeyboardEvents|P
  (params (Key :type Key%20Structure))
  (:Pressed
    (bind _asnon_game_instance_bp (Utilities|Casting|CastToNon_GameInstance_BP (Game|GetGameInstance)))
    (Utilities|FlowControl|FlipFlop
      (:A
        (Variables|/Game/Blueprints/NoN_GameInstance_BP.Non_GameInstance_BP_C|SetInventoryBag? _asnon_game_instance_bp false))
      (:B
        (Variables|/Game/Blueprints/NoN_GameInstance_BP.Non_GameInstance_BP_C|SetInventoryBag? _asnon_game_instance_bp true)))))

(event Input|MouseEvents|LeftMouseButton
  (params (Key :type Key%20Structure))
  (:Pressed
    (bind _asnon_game_instance_bp (Utilities|Casting|CastToNon_GameInstance_BP (Game|GetGameInstance)))
    (Development|PrintString (Utilities|GetDisplayName (Variables|/Game/Blueprints/NoN_GameInstance_BP.Non_GameInstance_BP_C|GetActorInHand _asnon_game_instance_bp)))))

(event Input|MouseEvents|MouseWheelUp
  (params (Key :type Key%20Structure))
  (:Pressed
    (bind _asnon_game_instance_bp (Utilities|Casting|CastToNon_GameInstance_BP (Game|GetGameInstance)))
    (Class|Pickup|MWUp(Message) (Variables|/Game/Blueprints/NoN_GameInstance_BP.Non_GameInstance_BP_C|GetCurrentBag _asnon_game_instance_bp))))

(event Input|MouseEvents|MouseWheelDown
  (params (Key :type Key%20Structure))
  (:Pressed
    (bind _asnon_game_instance_bp (Utilities|Casting|CastToNon_GameInstance_BP (Game|GetGameInstance)))
    (Class|Pickup|MWDown(Message) (Variables|/Game/Blueprints/NoN_GameInstance_BP.Non_GameInstance_BP_C|GetCurrentBag _asnon_game_instance_bp))))

(fn ConstructionScript)

(fn AddInteraction
  (params (Interaction :type BP%20Interact%20Object%20Object%20Reference))
  (bind _interactionlist (Variables|Default|GetInteractionList))
  (bind _interactiontimer (Variables|Default|GetInteractionTimer))
  (Utilities|Array|AddUnique _interactionlist Interaction)
  (if (> (Utilities|Array|Length _interactionlist) 0)
    (Utilities|Time|UnpauseTimerbyHandle _interactiontimer)
    (else
      (Utilities|Time|PauseTimerbyHandle _interactiontimer))))

(fn RemoveInteraction
  (params (Interaction :type BP%20Interact%20Object%20Object%20Reference))
  (bind _interactionlist (Variables|Default|GetInteractionList))
  (bind _interactiontimer (Variables|Default|GetInteractionTimer))
  (Utilities|Array|RemoveItem _interactionlist Interaction)
  (if (> (Utilities|Array|Length _interactionlist) 0)
    (Utilities|Time|UnpauseTimerbyHandle _interactiontimer)
    (else
      (Utilities|Time|PauseTimerbyHandle _interactiontimer)
      (Interaction|SetBestInteraction))))

(fn SetBestInteraction
  (params (Interaction :type BP%20Interact%20Object%20Object%20Reference))
  (bind _output_get (Variables|Default|SetNewInteraction Interaction))
  (Utilities|IsValid _output_get
    (:Is%20Valid
      (if (!= (Variables|Default|GetNewInteraction) (Variables|Default|GetSelected%20Interaction))
        (bind _selected_interaction (Variables|Default|GetSelected%20Interaction)
          (:then
            (Default|ToggleUI _selected_interaction false))
          (:else
            _))
        (bind _output_get_2 (Variables|Default|SetSelected%20Interaction (Variables|Default|GetNewInteraction)))
        (Default|ToggleUI _output_get_2 true)))
    (:Is%20Not%20Valid
      (bind _selected_interaction_2 (Variables|Default|GetSelected%20Interaction)
        (:then
          (Default|ToggleUI _selected_interaction_2 false)
          (Variables|Default|SetSelected%20Interaction 0))
        (:else)))))

(fn ShouldUpdateInteractions
  (return (and (> (Utilities|Array|Length (Variables|Default|GetInteractionList)) 0) (not (AI|Components|NavMovement|IsFalling (Variables|Character|GetCharacterMovement))))))

(fn GetBestInteraction
  (bind _dots (LocalVariables|GetDots))
  (bind _camera (Variables|Default|GetCamera))
  (bind (_indexofmaxvalue _maxvalue) (Math|Float|MaxOfFloatArray _dots))
  (for _array_element (Variables|Default|GetInteractionList)
    (Utilities|Array|Add (LocalVariables|GetDots) (Math|Vector|DotProduct (Math|Vector|Normalize (- (Transformation|GetWorldLocation (Variables|/Game/Blueprints/BP_InteractObject.BP_InteractObject_C|GetInteract_UI _array_element)) (Transformation|GetWorldLocation _camera))) (Math|Vector|GetForwardVector _camera))))
  (if (>= _maxvalue (Variables|Default|GetInteractTreshold))
    (Interaction|SetBestInteraction (Utilities|Array|Get(acopy) (Variables|Default|GetInteractionList) _indexofmaxvalue))
    (else
      (Interaction|SetBestInteraction))))

(fn UpdateInteraction
  (bind _shouldupdate_ (Interaction|ShouldUpdateInteractions))
  (if _shouldupdate_
    (Interaction|GetBestInteraction)
    (else
      (Interaction|SetBestInteraction))))